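; Inventory component that holds item slots, each pairing an item class with an amount.
; On BeginPlay it loads the inventory from BP_GameInstance, which it fetches through a lazily cached getter.
; AddItem appends a new slot without merging stacks, then saves the whole inventory back to the game instance.
; Helpers return the inventory or print each item's name and amount.
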(event `self.ReceiveBeginPlay`
  (bind _inventory (`/Game/Blueprints/Base/BP_GameInstance.GetInventory` (`self.GetDSGameInstance`)))
  (set `self.Inventory` _inventory))

(fn `AddItem`
  (params (ItemClass :type "/Game/Blueprints/InventorySystem/Items/BP_ItemBase Class Reference") (Amount :type Integer))
  (`KismetArrayLibrary.Array_Add` (`self.Inventory`) (make `/Game/Blueprints/InventorySystem/ST_InventorySlot` ItemClass Amount))
  (`/Game/Blueprints/Base/BP_GameInstance.SaveInventory` (`self.GetDSGameInstance`) (`self.Inventory`)))

(fn `GetDSGameInstance`
  (returns (GetDSGameInstance :type "/Game/Blueprints/Base/BP_GameInstance Object Reference"))
  (`self.GameInstance`
    (:`then`
      _)
    (:`else`
      (bind _asbp_game_instance (cast `/Game/Blueprints/Base/BP_GameInstance` (`GameplayStatics.GetGameInstance`)))
      (set `self.GameInstance` _asbp_game_instance)))
  (return (`self.GameInstance`)))

(fn `GetInventory`
  (returns (Inventory :type "Array of /Game/Blueprints/InventorySystem/ST_InventorySlot Structure"))
  (return (`self.Inventory`)))

(fn `PrintInventory`
  (for _array_element (`self.Inventory`)
    (bind _iteminfo_name (break `/Game/Blueprints/InventorySystem/ST_InventoryItem` (defaults `/Game/Blueprints/InventorySystem/BPC_Inventory` (break `/Game/Blueprints/InventorySystem/ST_InventorySlot` _array_element))))
    (`KismetSystemLibrary.PrintString` (`KismetStringLibrary.Concat_StrStr` (`KismetTextLibrary.Conv_TextToString` _iteminfo_name) ": " (`KismetStringLibrary.Conv_IntToString` (`.Amount_5_C22C891C40F6F1A97A08B28FF5E2D10D` (break `/Game/Blueprints/InventorySystem/ST_InventorySlot` _array_element)))))))